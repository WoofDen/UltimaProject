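; Player controller that sets up input and the gameplay HUD for a cursor-driven game with inventory and items.
; On local BeginPlay it adds the default Enhanced Input mapping context, shows the mouse cursor and creates the HUD if a pawn is possessed.
; Input actions call handlers for move-to-cursor, inventory toggle and item use.
; Pickup sends the item under the cursor to the player character's inventory, passing a huge amount.
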(event `self.ReceiveBeginPlay`
  (`parent.ReceiveBeginPlay`)
  (if (`self.IsLocalController`)
    (`|ExecutionSequence`
      (:`then_0`
        (`EnhancedInputSubsystemInterface.AddMappingContext` (subsystem `EnhancedInputLocalPlayerSubsystem`) "/Game/Input/IMC_Default.IMC_Default" 0 (struct))
        (set `self.bShowMouseCursor` true))
      (:`then_1`
        (`/Engine/EditorBlueprintResources/StandardMacros.IsValid` (`self.K2_GetPawn`)
          (:`Is Valid`
            (bind _returnvalue (`|CreateWidget` "/Game/Blueprints/UI/HUD/WBP_GameplayHUD.WBP_GameplayHUD_C" self))
            (`UserWidget.AddToViewport` _returnvalue 0)
            (set `self.GameUI` _returnvalue)))))))

(event `self.ReceivePossess`
  (params (PossessedPawn :type "Pawn Object Reference")))

(event `EnhancedInput|/Game/Input/Actions/IA_Move`
  (params (ActionValue :type Boolean) (ElapsedSeconds :type "Float (double-precision)") (TriggeredSeconds :type "Float (double-precision)") (InputAction :type "InputAction Object Reference" :default "/Game/Input/Actions/IA_Move.IA_Move"))
  (:`Triggered`
    (`self.MoveToCursor`)))

(event `EnhancedInput|/Game/Input/Actions/IA_InventoryToggle`
  (params (ActionValue :type Boolean) (ElapsedSeconds :type "Float (double-precision)") (TriggeredSeconds :type "Float (double-precision)") (InputAction :type "InputAction Object Reference" :default "/Game/Input/Actions/IA_InventoryToggle.IA_InventoryToggle"))
  (:`Triggered`
    (`self.HandleInventoryToggle`)))

(event `EnhancedInput|/Game/Input/Actions/IA_Pickup`
  (params (ActionValue :type Boolean) (ElapsedSeconds :type "Float (double-precision)") (TriggeredSeconds :type "Float (double-precision)") (InputAction :type "InputAction Object Reference" :default "/Game/Input/Actions/IA_Pickup.IA_Pickup"))
  (:`Triggered`
    (bind _asitem (cast `Item` (`InputHelpersFunctionLibrary.GetActorUnderCursor` self "ECC_WorldStatic")))
    (bind _asupcharacter (cast `UPCharacter` (`GameplayStatics.GetPlayerPawn` 0)))
    (`self.HandlePickupAction` _asitem 99999999 (`UPCharacter.GetInventoryComponent` _asupcharacter))))

(event `EnhancedInput|/Game/Input/Actions/IA_UseItem`
  (params (ActionValue :type Boolean) (ElapsedSeconds :type "Float (double-precision)") (TriggeredSeconds :type "Float (double-precision)") (InputAction :type "InputAction Object Reference" :default "/Game/Input/Actions/IA_UseItem.IA_UseItem"))
  (:`Triggered`
    (`self.HandleUseItem`)))

(fn `UserConstructionScript`)