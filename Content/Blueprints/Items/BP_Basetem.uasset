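; Base Blueprint for a world item that shows a mesh and a hover name widget.
; The construction script previews the mesh by synchronously loading the soft WorldMesh reference from DefaultStaticData.
; BeginPlay and OnItemDataChanged both call UpdateUI, which fills WBP_ItemName from ItemData and shows the HoverWidget.
; The UI update runs only when ItemData is valid and the instance is not the server.
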(event `self.ReceiveBeginPlay`
  (`parent.ReceiveBeginPlay`)
  (`self.UpdateUI`))

(event `self.OnItemDataChanged`
  (`self.UpdateUI`))

(fn `UpdateUI`
  (if (and (`KismetSystemLibrary.IsValid` (`self.ItemData`)) (not (`KismetSystemLibrary.IsServer`)))
    (bind _aswbp_item_name (cast `/Game/Blueprints/UI/Items/WBP_ItemName` (`WidgetComponent.GetWidget` (`self.HoverWidget`))))
    (`/Game/Blueprints/UI/Items/WBP_ItemName.InitFromItemData` _aswbp_item_name (`self.ItemData`))
    (`SceneComponent.SetVisibility` (`self.HoverWidget`) true true)))

(fn `UserConstructionScript`
  (bind _defaultstaticdata (`self.DefaultStaticData`))
  (bind _worldmesh (`ItemDataAsset.WorldMesh` _defaultstaticdata))
  ;[1 1 1] Load mesh preview
  (`/Engine/EditorBlueprintResources/StandardMacros.IsValid` _defaultstaticdata
    (:`Is Valid`
      (if (`KismetSystemLibrary.IsValidSoftObjectReference` _worldmesh)
        (bind _returnvalue (`KismetSystemLibrary.LoadAsset_Blocking` _worldmesh))
        (bind _asstatic_mesh (cast `StaticMesh` _returnvalue))
        (`StaticMeshComponent.SetStaticMesh` (`self.StaticMeshComponent`) _asstatic_mesh)))))