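; BP_Item_Common is an item Blueprint that shows a name widget for its item data.
; On BeginPlay and whenever the item data changes, it runs UpdateUI.
; UpdateUI skips the server, casts the HoverWidget component's widget to WBP_ItemName, initializes it from ItemData, then makes the component visible along with its children.
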(event `self.ReceiveBeginPlay`
  (`parent.ReceiveBeginPlay`)
  (`self.UpdateUI`))

(event `self.OnItemDataChanged`
  (`self.UpdateUI`))

(fn `UpdateUI`
  (if (not (`KismetSystemLibrary.IsServer`))
    (bind _aswbp_item_name (cast `/Game/Blueprints/UI/Items/WBP_ItemName` (`WidgetComponent.GetWidget` (`self.HoverWidget`))))
    (`/Game/Blueprints/UI/Items/WBP_ItemName.InitFromItemData` _aswbp_item_name (`self.ItemData`))
    (`SceneComponent.SetVisibility` (`self.HoverWidget`) true true)))

(fn `UserConstructionScript`)