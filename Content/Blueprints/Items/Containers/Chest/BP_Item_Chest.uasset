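; BP_Item_Chest is a chest container item that shows an interaction prompt widget when it is focused and accessible.
; The construction script hides the widget, and SetFocus toggles its visibility, requests a render update when shown, and prints the state for debugging.
; The container's items-changed handler is an empty stub, and the authority check on BeginPlay leads to no further logic.
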(event `self.ReceiveBeginPlay`
  (`parent.ReceiveBeginPlay`)
  (`/Engine/EditorBlueprintResources/ActorMacros.Switch Has Authority`))

(event `self.ContainerComponent.OnContainerItemsChanged`)

(event `self.SetFocus`
  (params (Focus :type Boolean) (IsAccessible :type Boolean))
  (bind _returnvalue (and IsAccessible Focus))
  (bind _interactionwidget (`self.InteractionWidget`))
  (`KismetSystemLibrary.PrintString` (`KismetStringLibrary.Conv_BoolToString` _returnvalue))
  (`SceneComponent.SetVisibility` _interactionwidget _returnvalue false)
  (if _returnvalue
    (`WidgetComponent.RequestRenderUpdate` _interactionwidget)))

(fn `UserConstructionScript`
  (`parent.UserConstructionScript`)
  (`SceneComponent.SetVisibility` (`self.InteractionWidget`) false false))