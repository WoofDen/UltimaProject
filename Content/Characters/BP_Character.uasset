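; BP_Character is a character Blueprint that uses the Gameplay Ability System and shows a stats HUD.
; On BeginPlay it applies the GE_TestCharacterInit effect to its own ability system component, then adds a WBP_MainStats widget for player controller 0 to the viewport.
; Each tick it rotates ControlRotationArrow to match the controller's control rotation whenever a controller is valid.
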(event `self.ReceiveBeginPlay`
  (`|ExecutionSequence`
    (:`then_0`
      (`AbilitySystemComponent.BP_ApplyGameplayEffectToSelf` :`self` (`AbilitySystemBlueprintLibrary.GetAbilitySystemComponent` self) :`GameplayEffectClass` "/Game/Effects/GE_TestCharacterInit.GE_TestCharacterInit_C" :`Level` 1.0))
    (:`then_1`
      (bind _returnvalue (`|CreateWidget` "/Game/UI/WBP_MainStats.WBP_MainStats_C" (`GameplayStatics.GetPlayerController` 0)))
      (`UserWidget.AddToViewport` _returnvalue 0))))

(event `self.ReceiveTick`
  (params (DeltaSeconds :type "Float (single-precision)"))
  (bind _returnvalue (`self.GetController`))
  (`/Engine/EditorBlueprintResources/StandardMacros.IsValid` _returnvalue
    (:`Is Valid`
      (`SceneComponent.K2_SetWorldRotation` (`self.ControlRotationArrow`) (`Controller.GetControlRotation` _returnvalue) false false))))

(fn `UserConstructionScript`)