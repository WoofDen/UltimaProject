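; BP_Basetem is a base item actor whose world appearance comes from an ItemDataAsset.
; Its construction script synchronously loads the soft-referenced DefaultStaticData, then that asset's soft WorldMesh, and applies it to the StaticMeshComponent as a preview.
; Each load runs only if its soft reference is valid, and the event graph holds no active logic.
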(fn `UserConstructionScript`
  (bind _defaultstaticdata (`self.DefaultStaticData`))
  ;[1 1 1] Load mesh preview
  (if (`KismetSystemLibrary.IsValidSoftObjectReference` _defaultstaticdata)
    (bind _returnvalue (`KismetSystemLibrary.LoadAsset_Blocking` _defaultstaticdata))
    (bind _asitem_data_asset (cast `ItemDataAsset` _returnvalue))
    (bind _worldmesh (`ItemDataAsset.WorldMesh` _asitem_data_asset))
    (if (`KismetSystemLibrary.IsValidSoftObjectReference` _worldmesh)
      (bind _returnvalue_2 (`KismetSystemLibrary.LoadAsset_Blocking` _worldmesh))
      (bind _asstatic_mesh (cast `StaticMesh` _returnvalue_2))
      (`StaticMeshComponent.SetStaticMesh` (`self.StaticMeshComponent`) _asstatic_mesh))))